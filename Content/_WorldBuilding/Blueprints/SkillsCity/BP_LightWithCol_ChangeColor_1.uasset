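; A light actor that changes its point light to a random color when something overlaps its box collider.
; Each overlap also prints the name of the overlapping actor, with no filtering by actor type.
; A separate LightSwitch event toggles the point light's visibility; nothing in this Blueprint calls it.
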(event OnComponentBeginOverlap(Box)
  (params (OverlappedComponent :type Primitive%20Component%20Object%20Reference) (OtherActor :type Actor%20Object%20Reference) (OtherComp :type Primitive%20Component%20Object%20Reference) (OtherBodyIndex :type Integer) (bFromSweep :type Boolean) (SweepResult :type Hit%20Result%20Structure%20%28by%20ref%29))
  (Development|PrintString (Utilities|String|Append "Collided With: " (Utilities|GetObjectName OtherActor)))
  (Rendering|Components|Light|SetLightColor (Variables|Default|GetPointLight) (Utilities|Struct|MakeLinearColor (Math|Random|RandomFloatinRange 0.0 1.0) (Math|Random|RandomFloatinRange 0.0 1.0) (Math|Random|RandomFloatinRange 0.0 1.0) 1.0) true))

(event EventBeginPlay)

(event Collision|EventActorBeginOverlap
  (params (OtherActor :type Actor%20Object%20Reference)))

(event EventTick
  (params (DeltaSeconds :type Float%20%28single-precision%29)))

(event EventLightSwitch
  (bind _pointlight (Variables|Default|GetPointLight))
  (Rendering|SetVisibility _pointlight (Class|KismetMathLibrary|XORBoolean (Variables|/Script/Engine.SceneComponent|GetbVisible _pointlight) true) false))

(fn ConstructionScript)