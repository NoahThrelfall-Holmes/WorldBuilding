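; BP_Ball is a physics-driven ball actor for a Breakout game.
; On each async physics tick, while the Sphere is simulating, it applies a small mass-scaled downward force along world Z.
; It also clamps the Sphere's linear velocity to a fixed maximum speed, with no minimum speed enforced.
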(event EventAsyncPhysicsTick
  (params (DeltaSeconds :type Float%20%28single-precision%29) (SimSeconds :type Float%20%28single-precision%29))
  (bind _sphere (Variables|Default|GetSphere))
  (bind _sphere_2 (Variables|Default|GetSphere))
  (if (Physics|IsSimulatingPhysics _sphere_2 "None")
    (Physics|AddForce _sphere (* (Physics|GetMass _sphere_2) "0.000000,0.000000,-2.000000") "None" false)
    (bind _returnvalue (Physics|GetPhysicsLinearVelocity _sphere "None"))
    (if (>= (Math|Vector|VectorLength _returnvalue) 2e+02)
      (Physics|SetPhysicsLinearVelocity _sphere (Math|Vector|ClampVectorSize _returnvalue 0.0 2e+02) false "None"))))

(fn ConstructionScript)